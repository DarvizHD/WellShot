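; Player controller for WellShot that handles menu, scoreboard and chat input and sets the pawn's player type.
; Input actions drive BP_WellShot_HUD widgets, switching cursor and pawn input for menu and chat, with the menu key closing open chat first.
; On possess, authority loads PlayerType from the "info" save and applies it to the character.
; Chat messages relay to GameState or GameMode, and GameMode messages rebroadcast through a dispatcher.
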(event Custom|Local%20Change%20Player%20Type
  (bind _returnvalue (SaveGame|LoadGamefromSlot "info"))
  (bind _asbp_well_shot_player_saved_info (Utilities|Casting|CastToBP_WellShot_PlayerSavedInfo _returnvalue))
  (CallFunction|ServerChangePlayerType (Variables|/Game/Start/BP_WellShot_PlayerSavedInfo.BP_WellShot_PlayerSavedInfo_C|GetPlayer%20Type _asbp_well_shot_player_saved_info)))

(event Custom|Server%20Change%20Player%20Type
  (params (PlayerType :type Boolean))
  (bind _asbp_well_shot_character (Utilities|Casting|CastToBP_WellShot_Character (Pawn|GetControlledPawn)))
  (Variables|/Game/Pawns/Character/BP_WellShot_Character.BP_WellShot_Character_C|SetPlayerType _asbp_well_shot_character PlayerType))

(event Custom|SendTo_PlayerController-GS
  (params (Sender :type String) (Message :type String))
  ;[1 1 1] to GameState
  (bind _asbp_well_shot_game_state (Utilities|Casting|CastToBP_WellShot_Game_State (Game|GetGameState)))
  (Default|OnMessageSendtoGSEvent _asbp_well_shot_game_state Sender Message))

(event Custom|HideChat
  ;[1 1 1] Show or Hide Chat
  (Default|HideChat (Variables|/Game/HUD/Chat/BP_ChatOnScreen.BP_ChatOnScreen_C|GetBP_ChatBox (Variables|/Game/HUD/BP_WellShot_HUD.BP_WellShot_HUD_C|GetChatOnScreen (Variables|Default|GetAs%20BP%20Well%20Shot%20HUD))))
  (Variables|Default|SetbShowMouseCursor false)
  (Input|SetInputModeGameOnly self false)
  (Input|EnableInput (Pawn|GetControlledPawn) self))

(event Custom|OnMessageSendToGM_Event
  (params (Sender :type String) (Message :type String) (ChatFlag :type Byte))
  ;[1 1 1] from GameMode
  (Default|CallOnMessageSendtoGM Sender Message ChatFlag))

(event Custom|SendTo_PlayerController-GM
  (params (Sender :type String) (Message :type String) (ChatFlag :type Byte))
  ;[1 1 1] to GameMode
  (bind _asbp_well_shot_game_mode (Utilities|Casting|CastToBP_WellShot_Game_Mode (Game|GetGameMode)))
  (Default|SendtoGameMode _asbp_well_shot_game_mode Sender Message ChatFlag))

(event Input|EnhancedActionEvents|EnhancedInputActionIA_Main_Menu
  (params (ActionValue :type Boolean) (ElapsedSeconds :type Float%20%28double-precision%29) (TriggeredSeconds :type Float%20%28double-precision%29) (InputAction :type Input%20Action%20Object%20Reference :default "/Game/Inputs/IA_Main_Menu.IA_Main_Menu"))
  ;[1 1 1] If Chat is opened
  (if (== (Variables|/Script/UMG.WidgetSwitcher|GetActiveWidgetIndex (Variables|/Game/HUD/Chat/BP_ChatBox.BP_ChatBox_C|GetWidgetSwitcher_0 (Variables|/Game/HUD/Chat/BP_ChatOnScreen.BP_ChatOnScreen_C|GetBP_ChatBox (Variables|/Game/HUD/BP_WellShot_HUD.BP_WellShot_HUD_C|GetChatOnScreen (Variables|Default|GetAs%20BP%20Well%20Shot%20HUD))))) 1)
    (CallFunction|HideChat)
    (else
      (Utilities|FlowControl|FlipFlop
        (:A
          (Default|DrawMainMenu (Variables|Default|GetAs%20BP%20Well%20Shot%20HUD))
          (Variables|Default|SetbShowMouseCursor true)
          (Input|DisableInput (Pawn|GetControlledPawn) self))
        (:B
          (Default|DeleteMainMenu (Variables|Default|GetAs%20BP%20Well%20Shot%20HUD))
          (Variables|Default|SetbShowMouseCursor false)
          (Input|EnableInput (Pawn|GetControlledPawn) self))))))

(event Input|EnhancedActionEvents|EnhancedInputActionIA_Chat
  (params (ActionValue :type Boolean) (ElapsedSeconds :type Float%20%28double-precision%29) (TriggeredSeconds :type Float%20%28double-precision%29) (InputAction :type Input%20Action%20Object%20Reference :default "/Game/Inputs/IA_Chat.IA_Chat"))
  (bind _as_bp_well_shot_hud (Variables|Default|GetAs%20BP%20Well%20Shot%20HUD))
  (bind _chatonscreen (Variables|/Game/HUD/BP_WellShot_HUD.BP_WellShot_HUD_C|GetChatOnScreen _as_bp_well_shot_hud))
  (bind _bp_chatbox (Variables|/Game/HUD/Chat/BP_ChatOnScreen.BP_ChatOnScreen_C|GetBP_ChatBox _chatonscreen))
  ;[1 1 1] Show or Hide Chat
  (if (== (Variables|/Script/UMG.WidgetSwitcher|GetActiveWidgetIndex (Variables|/Game/HUD/Chat/BP_ChatBox.BP_ChatBox_C|GetWidgetSwitcher_0 _bp_chatbox)) 0)
    (Default|ShowChat _bp_chatbox)
    (Variables|Default|SetbShowMouseCursor true)
    (Input|SetInputModeGameandUI self (Variables|/Game/HUD/Chat/BP_ChatBox.BP_ChatBox_C|GetEditableTextBox_ChatLine _bp_chatbox) "DoNotLock" true false)
    (Input|DisableInput (Pawn|GetControlledPawn) self)
    (else
      (Default|HideChat _bp_chatbox)
      (Variables|Default|SetbShowMouseCursor false)
      (Input|SetInputModeGameOnly self false)
      (Input|EnableInput (Pawn|GetControlledPawn) self))))

(event Input|EnhancedActionEvents|EnhancedInputActionIA_Score_Board
  (params (ActionValue :type Boolean) (ElapsedSeconds :type Float%20%28double-precision%29) (TriggeredSeconds :type Float%20%28double-precision%29) (InputAction :type Input%20Action%20Object%20Reference :default "/Game/Inputs/IA_Score_Board.IA_Score_Board"))
  (:Started
    (Default|ShowScoreBoard (Variables|Default|GetAs%20BP%20Well%20Shot%20HUD)))
  (:Completed
    (Default|CloseScoreBoard (Variables|Default|GetAs%20BP%20Well%20Shot%20HUD))))

(event EventPossess
  (params (PossessedPawn :type Pawn%20Object%20Reference))
  (Networking|SwitchHasAuthority
    (:Authority
      (CallFunction|LocalChangePlayerType))))

(event EventBeginPlay
  (Input|SetInputModeGameOnly self false)
  (bind _asbp_well_shot_hud (Utilities|Casting|CastToBP_WellShot_HUD (HUD|GetHUD)))
  (Variables|Default|SetAs%20BP%20Well%20Shot%20HUD _asbp_well_shot_hud))

(fn ConstructionScript)

(fn SetMesh
  (params (Player%20Type :type Boolean))
  (CallFunction|ServerChangePlayerType Player%20Type))