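; Game mode for WellShot that handles player respawning and relays chat messages to connected players.
; Respawn destroys the controller's current pawn, then spawns and possesses a new BP_WellShot_Character at a random PlayerStart.
; Messages are forwarded to each player controller through the game state's player array.
; On logout, the departing player's name is broadcast with a disconnect notice.
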(event Custom|Respawn
  (params (My_Controller :type Controller%20Object%20Reference))
  (bind _returnvalue (Pawn|GetControlledPawn My_Controller))
  (bind _outactors (Actor|GetAllActorsOfClass "/Script/Engine.PlayerStart"))
  (Utilities|IsValid _returnvalue
    (:Is%20Valid
      (Actor|DestroyActor _returnvalue))
    (:Is%20Not%20Valid
      _))
  (bind _returnvalue_2 (Game|SpawnActorfromClass "/Game/Pawns/Character/BP_WellShot_Character.BP_WellShot_Character_C" (Transformation|GetActorTransform (Utilities|Array|Get(acopy) _outactors (Math|Random|RandomIntegerinRange 0 (- (Utilities|Array|Length _outactors) 1)))) "AdjustIfPossibleButAlwaysSpawn" "MultiplyWithRoot" 0 0))
  (Pawn|Possess My_Controller _returnvalue_2))

(event Custom|SendTo_GameMode
  (params (Sender :type String) (Message :type String) (ChatFlag :type Byte))
  (for _array_element (Variables|/Script/Engine.GameStateBase|GetPlayerArray (Game|GetGameState))
    (bind _asbp_well_shot_player_controller (Utilities|Casting|CastToBP_WellShot_Player_Controller (Game|GetPlayerController _array_element)))
    (Default|OnMessageSendtoGMEvent _asbp_well_shot_player_controller Sender Message ChatFlag)))

(event EventBeginPlay)

(event EventTick
  (params (DeltaSeconds :type Float%20%28single-precision%29)))

(event EventOnLogout
  (params (ExitingController :type Controller%20Object%20Reference))
  (bind _asbp_well_shot_player_state (Utilities|Casting|CastToBP_WellShot_Player_State (Variables|/Script/Engine.Controller|GetPlayerState ExitingController)))
  (CallFunction|SendtoGameMode (Utilities|String|ToString(Text) (Variables|/Game/States/BP_WellShot_Player_State.BP_WellShot_Player_State_C|GetMyName _asbp_well_shot_player_state)) "Disconnected from server" 2))

(fn ConstructionScript)