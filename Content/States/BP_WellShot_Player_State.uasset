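; BP_WellShot_Player_State is a player state that tracks a player's name, kills, deaths and dead flag in WellShot.
; On BeginPlay, if player controller 0 is local, it loads the saved name from the "info" slot and passes it to SendMyNameToServer.
; That event stores the name and has the game mode post a "Connected to server" chat message.
; AddKill and AddDeath update the counters, and AddDeath also marks the player dead.
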(event Custom|AddKill
  (Math|Integer|IncrementInt (Variables|Default|GetMyKills)))

(event Custom|AddDeath
  (Math|Integer|IncrementInt (Variables|Default|GetMyDeaths)
    (:%20%20
      (Variables|Default|SetisDead true))))

(event Custom|Send%20My%20Name%20To%20Server
  (params (MyName :type Text))
  (Variables|Default|SetMyName MyName)
  (bind _asbp_well_shot_game_mode (Utilities|Casting|CastToBP_WellShot_Game_Mode (Game|GetGameMode)))
  (Default|SendtoGameMode _asbp_well_shot_game_mode (Utilities|String|ToString(Text) (Variables|Default|GetMyName)) "Connected to server" 1))

(event EventBeginPlay
  (if (Pawn|IsLocalPlayerController (Game|GetPlayerController 0))
    (bind _returnvalue (SaveGame|LoadGamefromSlot "info"))
    (bind _asbp_well_shot_player_saved_info (Utilities|Casting|CastToBP_WellShot_PlayerSavedInfo _returnvalue))
    (CallFunction|SendMyNametoServer (Variables|/Game/Start/BP_WellShot_PlayerSavedInfo.BP_WellShot_PlayerSavedInfo_C|GetPlayer%20Name _asbp_well_shot_player_saved_info))))

(event EventTick
  (params (DeltaSeconds :type Float%20%28single-precision%29)))

(fn ConstructionScript)