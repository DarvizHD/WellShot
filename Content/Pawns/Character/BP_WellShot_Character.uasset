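; Player character for the WellShot multiplayer shooter, with rifle, ammo, health and left/right shoulder camera switching.
; Shooting is rate-limited and line-traces from the camera, applying damage after a hit on a "pawn"-tagged actor.
; Death records kill and death in player states, removes the HUD, ragdolls, then requests a delayed game-mode respawn.
; Server and multicast events relay camera and audio; RepNotifies broadcast HP and ammo and update the mesh.
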(event Custom|Server1
  ;[0 0.9594 0.03886] SHOT
  (if (Variables|Default|GetCan%20Shoot)
    (if (> (Variables|Default|GetAMMO) 0)
      (CallFunction|AudioMulticast "/Game/Audio/shoot.shoot")
      (Variables|Default|SetCan%20Shoot false)
      (Variables|Default|SetAMMO (- (Variables|Default|GetAMMO) 1))
      (CallFunction|TracefromClient)
      (Utilities|FlowControl|Delay 0.3)
      (Variables|Default|SetCan%20Shoot true)
      (else
        (CallFunction|AudioMulticast "/Game/Audio/no-ammo.no-ammo")))))

(event Custom|Ragdoll
  ;[1 0 0.007763] DAMAGE
  (Components|DestroyComponent (Variables|Default|GetCapsuleComponent))
  (Physics|SetSimulatePhysics (Variables|Character|GetMesh) true))

(event Custom|Trace%20From%20Client
  ;[0 0.9594 0.03886] SHOT
  (bind _hit_actor (CallFunction|TRACE))
  (if (Actor|ActorHasTag _hit_actor "pawn")
    (CallFunction|ShootfromServer)))

(event Custom|Shoot%20From%20Server
  ;[0 0.9594 0.03886] SHOT
  (bind _hit_actor (CallFunction|TRACE))
  (Game|Damage|ApplyDamage _hit_actor 25.0 (Pawn|GetController) 0))

(event Custom|Add%20Score
  ;[1 0 0.007763] DAMAGE
  (bind _asbp_well_shot_player_state (Utilities|Casting|CastToBP_WellShot_Player_State (Variables|Default|GetPlayerState)))
  (Default|AddDeath _asbp_well_shot_player_state)
  (bind _asbp_well_shot_player_state_2 (Utilities|Casting|CastToBP_WellShot_Player_State (Variables|/Script/Engine.Controller|GetPlayerState (stale Game|Damage|EventAnyDamage InstigatedBy))))
  (Default|AddKill _asbp_well_shot_player_state_2))

(event Custom|Recharge
  (Variables|Default|SetAMMO 25))

(event Custom|Right%20Camera%20Server
  ;[1 1 1] Change Camera
  (CallFunction|RightCameraMulticast))

(event Custom|own
  (bind _returnvalue (Pawn|GetController))
  ;[1 1 1] Draw UI
  (if (Pawn|IsLocalController _returnvalue)
    (bind _asbp_well_shot_player_controller (Utilities|Casting|CastToBP_WellShot_Player_Controller _returnvalue))
    (bind _asbp_well_shot_hud (Utilities|Casting|CastToBP_WellShot_HUD (HUD|GetHUD _asbp_well_shot_player_controller)))
    (Default|DrawUI _asbp_well_shot_hud)))

(event Custom|Left%20Camera%20Server
  ;[1 1 1] Change Camera
  (CallFunction|LeftCameraMulticast))

(event Custom|own2
  ;[1 0 0.007763] DAMAGE
  (bind _asbp_well_shot_player_controller (Utilities|Casting|CastToBP_WellShot_Player_Controller (Pawn|GetController)))
  (bind _asbp_well_shot_hud (Utilities|Casting|CastToBP_WellShot_HUD (HUD|GetHUD _asbp_well_shot_player_controller)))
  (Default|DeleteUI _asbp_well_shot_hud))

(event Custom|Left%20Camera%20Multicast
  ;[1 1 1] Change Camera
  (Transformation|SetRelativeLocation (Variables|Default|GetCamera) "110.000000,-60.000000,70.000000" false false))

(event Custom|Right%20Camera%20Multicast
  ;[1 1 1] Change Camera
  (Transformation|SetRelativeLocation (Variables|Default|GetCamera) "110.000000,60.000000,70.000000" false false))

(event Custom|Audio%20Server
  (params (Audio%20S :type Sound%20Base%20Object%20Reference))
  ;[1 1 1] Audio
  (CallFunction|AudioMulticast Audio%20S))

(event Custom|Audio%20Multicast
  (params (Audio%20M :type Sound%20Base%20Object%20Reference))
  ;[1 1 1] Audio
  (bind _returnvalue (Audio|SpawnSoundAttached Audio%20M (Variables|Default|GetCapsuleComponent) "None" "0, 0, 0" "0, 0, 0" "KeepRelativeOffset" false 1.0 1.0 0.0 "/Game/Audio/WellShot_SoundAttenuation.WellShot_SoundAttenuation" 0))
  (Audio|Components|Audio|Play _returnvalue 0.0))

(event Input|EnhancedActionEvents|EnhancedInputActionIA_Shoot
  (params (ActionValue :type Boolean) (ElapsedSeconds :type Float%20%28double-precision%29) (TriggeredSeconds :type Float%20%28double-precision%29) (InputAction :type Input%20Action%20Object%20Reference :default "/Game/Inputs/IA_Shoot.IA_Shoot"))
  ;[0 0.9594 0.03886] SHOT
  (CallFunction|Server1))

(event Input|EnhancedActionEvents|EnhancedInputActionIA_Left_Camera
  (params (ActionValue :type Boolean) (ElapsedSeconds :type Float%20%28double-precision%29) (TriggeredSeconds :type Float%20%28double-precision%29) (InputAction :type Input%20Action%20Object%20Reference :default "/Game/Inputs/IA_Left_Camera.IA_Left_Camera"))
  ;[1 1 1] Change Camera
  (CallFunction|LeftCameraServer))

(event Input|EnhancedActionEvents|EnhancedInputActionIA_Right_Camera
  (params (ActionValue :type Boolean) (ElapsedSeconds :type Float%20%28double-precision%29) (TriggeredSeconds :type Float%20%28double-precision%29) (InputAction :type Input%20Action%20Object%20Reference :default "/Game/Inputs/IA_Right_Camera.IA_Right_Camera"))
  ;[1 1 1] Change Camera
  (CallFunction|RightCameraServer))

(event Input|EnhancedActionEvents|EnhancedInputActionIA_Recharge
  (params (ActionValue :type Boolean) (ElapsedSeconds :type Float%20%28double-precision%29) (TriggeredSeconds :type Float%20%28double-precision%29) (InputAction :type Input%20Action%20Object%20Reference :default "/Game/Inputs/IA_Recharge.IA_Recharge"))
  (CallFunction|Recharge))

(event Game|Damage|EventAnyDamage
  (params (Damage :type Float%20%28single-precision%29) (DamageType :type Damage%20Type%20Object%20Reference) (InstigatedBy :type Controller%20Object%20Reference) (DamageCauser :type Actor%20Object%20Reference))
  ;[1 0 0.007763] DAMAGE
  (if (not (Variables|Default|Getyou%20can't%20shoot%20me))
    (bind _output_get (Variables|Default|SetHP (- (Variables|Default|GetHP) Damage)))
    (if (<= _output_get 0.0)
      (Variables|Default|Setyou%20can't%20shoot%20me true)
      (Variables|Default|SetCan%20Shoot false)
      (CallFunction|Own2)
      (CallFunction|AddScore)
      (CallFunction|Ragdoll)
      (Utilities|FlowControl|Delay 5.0)
      (bind _asbp_well_shot_game_mode (Utilities|Casting|CastToBP_WellShot_Game_Mode (Game|GetGameMode)))
      (Default|Respawn _asbp_well_shot_game_mode (Game|GetInstigatorController)))))

(event EventPossessed
  (params (NewController :type Controller%20Object%20Reference))
  ;[1 1 1] Draw UI
  (bind _asbp_well_shot_player_state (Utilities|Casting|CastToBP_WellShot_Player_State (Variables|Default|GetPlayerState)))
  (Variables|/Game/States/BP_WellShot_Player_State.BP_WellShot_Player_State_C|SetisDead _asbp_well_shot_player_state false)
  (Utilities|FlowControl|Delay 1.0)
  (CallFunction|Own))

(event EventBeginPlay
  ;[1 1 1] Change Player Type(Mesh)
  (CallFunction|UpdateMesh))

(fn ConstructionScript
  (Transformation|AttachComponentToComponent (Variables|Default|GetAssault_Rifle_A) (Variables|Character|GetMesh) "WeaponSocket" "KeepRelative" "KeepRelative" "KeepRelative" true))

(fn OnRepHP
  (Default|CallOnHPchanged (Variables|Default|GetHP)))

(fn OnRepAMMO
  (Default|CallOnAMMOchanged (Variables|Default|GetAMMO)))

(fn TRACE
  (bind _camera (Variables|Default|GetCamera))
  (bind _returnvalue (Transformation|GetWorldLocation _camera))
  (bind _outhit (Collision|LineTraceByChannel _returnvalue (+ _returnvalue (* (Math|Vector|GetForwardVector _camera) 3e+04)) "TraceTypeQuery1" false 0 "None"))
  (return (.HitActor (Collision|BreakHitResult _outhit))))

(fn UpdateMesh
  (Components|SkeletalMesh|SetSkeletalMeshAsset (Variables|Character|GetMesh) (select (Variables|Default|GetPlayerType) "/Game/Pawns/Character/Ch15_nonPBR.Ch15_nonPBR" "/Game/Pawns/Character2/Swat.Swat")))

(fn OnRepPlayerType
  (CallFunction|UpdateMesh))