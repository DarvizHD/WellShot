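; BP_WellShot_HUD is the player HUD that creates and toggles WellShot's on-screen widgets: chat, FPS counter, game UI, main menu and scoreboard.
; On BeginPlay it adds chat, creates the FPS counter and shows it according to the ShowFPS setting loaded from the "info" save slot.
; Events add or remove each widget, with the main menu also switching input between game-and-UI and game-only modes.
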(event Custom|drawUI
  ;[1 1 1] GameUI
  (bind _returnvalue (UserInterface|CreateWidget "/Game/HUD/BP_WellShot_UMG.BP_WellShot_UMG_C" (Variables|Default|GetPlayerOwner)))
  (bind _output_get (Variables|Default|SetUI _returnvalue))
  (UserInterface|Viewport|AddtoViewport _output_get 0))

(event Custom|deleteUI
  ;[1 1 1] GameUI
  (Widget|RemovefromParent (Variables|Default|GetUI))
  (Variables|Default|SetUI 0))

(event Custom|Draw%20Main%20Menu
  (bind _all_umg (Variables|Default|GetAll_UMG))
  (bind _bp_main_menu (Variables|/Game/HUD/All_UMG.All_UMG_C|GetBP_Main_Menu _all_umg))
  (UserInterface|Viewport|AddtoViewport _bp_main_menu 0)
  (Input|SetInputModeGameandUI (Game|Player|GetOwningPlayerController) _bp_main_menu "DoNotLock" false false))

(event Custom|Delete%20Main%20Menu
  (Widget|RemovefromParent (Variables|/Game/HUD/All_UMG.All_UMG_C|GetBP_Main_Menu (Variables|Default|GetAll_UMG)))
  (Input|SetInputModeGameOnly (Game|Player|GetOwningPlayerController) false))

(event Custom|ShowFPS
  ;[1 1 1] FPS UI
  (UserInterface|Viewport|AddtoViewport (Variables|Default|GetFPS) 0))

(event Custom|DeleteFPS
  ;[1 1 1] FPS UI
  (Widget|RemovefromParent (Variables|Default|GetFPS)))

(event Custom|Show%20Score%20Board
  (bind _returnvalue (UserInterface|CreateWidget "/Game/HUD/BP_ScoreBoard.BP_ScoreBoard_C" (Variables|Default|GetPlayerOwner)))
  (UserInterface|Viewport|AddtoViewport _returnvalue 0))

(event Custom|Close%20Score%20Board
  (Widget|RemovefromParent (stale Custom|Show%20Score%20Board _returnvalue)))

(event EventBeginPlay
  (bind _playerowner (Variables|Default|GetPlayerOwner))
  ;[1 1 1] Chat UI
  (bind _returnvalue (UserInterface|CreateWidget "/Game/HUD/Chat/BP_ChatOnScreen.BP_ChatOnScreen_C" _playerowner))
  (bind _output_get (Variables|Default|SetChatOnScreen _returnvalue))
  (UserInterface|Viewport|AddtoViewport _output_get 0)
  ;[1 1 1] FPS UI
  (bind _returnvalue_2 (UserInterface|CreateWidget "/Game/HUD/BP_ShowFPS.BP_ShowFPS_C" _playerowner))
  (Variables|Default|SetFPS _returnvalue_2)
  (bind _returnvalue_3 (SaveGame|LoadGamefromSlot "info"))
  (bind _asbp_well_shot_player_saved_info (Utilities|Casting|CastToBP_WellShot_PlayerSavedInfo _returnvalue_3))
  (if (Variables|/Game/Start/BP_WellShot_PlayerSavedInfo.BP_WellShot_PlayerSavedInfo_C|GetShow%20FPS _asbp_well_shot_player_saved_info)
    (UserInterface|Viewport|AddtoViewport (Variables|Default|GetFPS) 0)
    (else
      (Widget|RemovefromParent (Variables|Default|GetFPS)))))

(fn ConstructionScript)